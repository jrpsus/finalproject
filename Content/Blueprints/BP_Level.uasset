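; BP_Level sets up the UI and hint text for each level of a puzzle game about a sphere and colored platforms.
; On BeginPlay it adds the WB_Level widget to the viewport and enables game-and-UI input with a visible mouse cursor.
; A branch chain on the current level name then sets LevelHintText for level1 through level6, with the last left blank.
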(event `self.ReceiveBeginPlay`
  (bind _returnvalue (`GameplayStatics.GetPlayerController` 0))
  (bind _returnvalue_2 (`|CreateWidget` "/Game/Blueprints/WB_Level.WB_Level_C"))
  (`UserWidget.AddToViewport` _returnvalue_2 0)
  (`WidgetBlueprintLibrary.SetInputMode_GameAndUIEx` _returnvalue null "DoNotLock" false)
  (set `PlayerController.bShowMouseCursor` true _returnvalue)
  (bind _returnvalue_3 (`GameplayStatics.GetCurrentLevelName` true))
  (if (`KismetStringLibrary.EqualEqual_StrStr` _returnvalue_3 "level1")
    (set `self.Level Hint Text` "Click on the white platforms to remove them.")
    (elif (`KismetStringLibrary.EqualEqual_StrStr` _returnvalue_3 "level2")
      (set `self.Level Hint Text` "Don't let the sphere touch red.")
      (elif (`KismetStringLibrary.EqualEqual_StrStr` _returnvalue_3 "level3")
        (set `self.Level Hint Text` "Purple platforms are bouncy.")
        (elif (`KismetStringLibrary.EqualEqual_StrStr` _returnvalue_3 "level4")
          (set `self.Level Hint Text` "Yellow cubes have the same physics as the sphere.")
          (elif (`KismetStringLibrary.EqualEqual_StrStr` _returnvalue_3 "level5")
            (set `self.Level Hint Text` "Some blue platforms automatically rotate.")
            (elif (`KismetStringLibrary.EqualEqual_StrStr` _returnvalue_3 "level6")
              (set `self.Level Hint Text` ""))))))))

(fn `UserConstructionScript`)